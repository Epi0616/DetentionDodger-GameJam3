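; BP_Car is a moving car hazard that shuttles back and forth along the Y axis and kills the player on contact.
; Tick moves the capsule by a fixed, non-delta-scaled step, then line-traces along forward and backward vectors for WorldStatic objects.
; Either hit triggers a shared FlipFlop that reverses MoveDirection.
; Front and back collision overlaps halt the car, call KillPlayer on the third-person character, then resume movement after a delay.
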(event OnComponentBeginOverlap(BackCollision)
  (params (OverlappedComponent :type Primitive%20Component%20Object%20Reference) (OtherActor :type Actor%20Object%20Reference) (OtherComp :type Primitive%20Component%20Object%20Reference) (OtherBodyIndex :type Integer) (bFromSweep :type Boolean) (SweepResult :type Hit%20Result%20Structure%20%28by%20ref%29))
  (if (Actor|ActorHasTag OtherActor "Player")
    (Variables|Default|SetcanMove false)
    (bind _asbp_third_person_character (Utilities|Casting|CastToBP_ThirdPersonCharacter OtherActor))
    (Default|KillPlayer _asbp_third_person_character)
    (Utilities|FlowControl|Delay 3.0)
    (Variables|Default|SetcanMove true)))

(event OnComponentBeginOverlap(FrontCollision)
  (params (OverlappedComponent :type Primitive%20Component%20Object%20Reference) (OtherActor :type Actor%20Object%20Reference) (OtherComp :type Primitive%20Component%20Object%20Reference) (OtherBodyIndex :type Integer) (bFromSweep :type Boolean) (SweepResult :type Hit%20Result%20Structure%20%28by%20ref%29))
  (if (Actor|ActorHasTag OtherActor "Player")
    (Variables|Default|SetcanMove false)
    (bind _asbp_third_person_character (Utilities|Casting|CastToBP_ThirdPersonCharacter OtherActor))
    (Default|KillPlayer _asbp_third_person_character)
    (Utilities|FlowControl|Delay 3.0)
    (Variables|Default|SetcanMove true)))

(event EventTick
  (params (DeltaSeconds :type Float%20%28single-precision%29))
  (bind _returnvalue (Transformation|GetActorLocation))
  (bind _returnvalue_2 (Transformation|GetActorLocation))
  ;[1 1 1] Car Movement
  (Utilities|FlowControl|Sequence
    (:then_0
      (if (Variables|Default|GetcanMove)
        ;;[1 1 1] Move the "Car"
        (Transformation|AddRelativeLocation (Variables|Collision|GetCapsuleComponent) (* (Variables|Default|GetMoveDirection) (Variables|Default|GetMoveSpeed)) false false)))
    (:then_1
      ;;[0 0.0311 1] Left Side Check
      (bind _returnvalue_3 (Collision|LineTraceForObjects _returnvalue_2 (+ _returnvalue_2 (* (Transformation|GetActorForwardVector) 1.5e+02)) (Utilities|Array|MakeArray "ObjectTypeQuery1") false 0 "ForDuration" true "(R=0.000000,G=0.044782,B=1.000000,A=1.000000)"))
      (if _returnvalue_3
        ;;[1 1 1] Change Direction
        (Utilities|FlowControl|FlipFlop :!label _label
          (:A
            (Variables|Default|SetMoveDirection "0.000000,-1.000000,0.000000"))
          (:B
            (Variables|Default|SetMoveDirection "0.000000,1.000000,0.000000")))))
    (:then_2
      ;;[1 0 0.02387] Right Side Check
      (bind _returnvalue_4 (Collision|LineTraceForObjects _returnvalue (+ _returnvalue (* (* (Transformation|GetActorForwardVector) -1.0) 1.5e+02)) (Utilities|Array|MakeArray "ObjectTypeQuery1") false 0 "ForDuration"))
      (if _returnvalue_4
        (goto _label)))))

(fn ConstructionScript)