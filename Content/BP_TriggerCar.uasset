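; A traffic car hazard that kills the player on contact and loops along a straight path.
; On BeginPlay it stores its spawn point and picks one of five random car meshes with matching materials.
; Tick moves the capsule along a set direction while movement is allowed.
; Front and back collision overlaps kill a tagged player, pausing the car briefly, or teleport it back to spawn upon reaching its end trigger.
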(event OnComponentBeginOverlap(BackCollision)
  (params (OverlappedComponent :type Primitive%20Component%20Object%20Reference) (OtherActor :type Actor%20Object%20Reference) (OtherComp :type Primitive%20Component%20Object%20Reference) (OtherBodyIndex :type Integer) (bFromSweep :type Boolean) (SweepResult :type Hit%20Result%20Structure%20%28by%20ref%29))
  ;[1 1 1] Player Detection On Cars
  (Utilities|FlowControl|Sequence
    (:then_0
      (if (Actor|ActorHasTag OtherActor "Player")
        (Variables|Default|SetcanMove false)
        (bind _asbp_third_person_character (Utilities|Casting|CastToBP_ThirdPersonCharacter OtherActor))
        (Default|KillPlayer _asbp_third_person_character)
        (Utilities|FlowControl|Delay 3.0)
        (Variables|Default|SetcanMove true)))
    (:then_1
      (if (== OtherActor (Variables|Default|GetEndTrigger))
        (Transformation|SetActorLocation (Variables|Default|GetspawnPoint) false false)))))

(event OnComponentBeginOverlap(FrontCollision)
  (params (OverlappedComponent :type Primitive%20Component%20Object%20Reference) (OtherActor :type Actor%20Object%20Reference) (OtherComp :type Primitive%20Component%20Object%20Reference) (OtherBodyIndex :type Integer) (bFromSweep :type Boolean) (SweepResult :type Hit%20Result%20Structure%20%28by%20ref%29))
  ;[1 1 1] Player Detection On Cars
  (Utilities|FlowControl|Sequence
    (:then_0
      (if (Actor|ActorHasTag OtherActor "Player")
        (Variables|Default|SetcanMove false)
        (bind _asbp_third_person_character (Utilities|Casting|CastToBP_ThirdPersonCharacter OtherActor))
        (Default|KillPlayer _asbp_third_person_character)
        (Utilities|FlowControl|Delay 3.0)
        (Variables|Default|SetcanMove true)))
    (:then_1
      (if (== OtherActor (Variables|Default|GetEndTrigger))
        (Transformation|SetActorLocation (Variables|Default|GetspawnPoint) false false)))))

(event EventBeginPlay
  (Variables|Default|SetspawnPoint (Transformation|GetActorLocation))
  (switch int (Math|Random|RandomIntegerinRange 0 4)
    (:0
      (Components|StaticMesh|SetStaticMesh (Variables|Default|GetCar%20Body) "/Game/CarAssets/Cars/BlueCar/BlueCar.BlueCar")
      (Rendering|Material|SetMaterial (Variables|Default|GetCar%20Body) 0 "/Game/CarAssets/Cars/BlueCar/M_BlueCar.M_BlueCar"))
    (:1
      (Components|StaticMesh|SetStaticMesh (Variables|Default|GetCar%20Body) "/Game/CarAssets/Cars/GreenCar/GreenCar.GreenCar")
      (Rendering|Material|SetMaterial (Variables|Default|GetCar%20Body) 0 "/Game/CarAssets/Cars/GreenCar/M_GreenCar.M_GreenCar"))
    (:2
      (Components|StaticMesh|SetStaticMesh (Variables|Default|GetCar%20Body) "/Game/CarAssets/Cars/PoliceCar/PoliceCar.PoliceCar")
      (Rendering|Material|SetMaterial (Variables|Default|GetCar%20Body) 0 "/Game/CarAssets/Cars/PoliceCar/M_PoliceCar.M_PoliceCar"))
    (:3
      (Components|StaticMesh|SetStaticMesh (Variables|Default|GetCar%20Body) "/Game/CarAssets/Cars/RedCar/RedCar.RedCar")
      (Rendering|Material|SetMaterial (Variables|Default|GetCar%20Body) 0 "/Game/CarAssets/Cars/RedCar/M_RedCar.M_RedCar"))
    (:4
      (Components|StaticMesh|SetStaticMesh (Variables|Default|GetCar%20Body) "/Game/CarAssets/Cars/TaxiCar/TaxiCar.TaxiCar")
      (Rendering|Material|SetMaterial (Variables|Default|GetCar%20Body) 0 "/Game/CarAssets/Cars/TaxiCar/M_TaxiCar.M_TaxiCar"))))

(event EventTick
  (params (DeltaSeconds :type Float%20%28single-precision%29))
  ;[1 1 1] Car Movement
  (Utilities|FlowControl|Sequence
    (:then_0
      (if (Variables|Default|GetcanMove)
        ;;[1 1 1] Move the "Car"
        (Transformation|AddRelativeLocation (Variables|Collision|GetCapsuleComponent) (* (Variables|Default|GetMoveDirection) (Variables|Default|GetMoveSpeed)) false false)))))

(fn ConstructionScript)